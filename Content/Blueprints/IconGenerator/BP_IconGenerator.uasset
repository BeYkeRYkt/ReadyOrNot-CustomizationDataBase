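; Icon generator actor that renders character customization items from a data table into preview icon textures, using editor-only asset saving.
; On BeginPlay, delayed loops step through each row, first loading meshes and materials onto temp components to prestream textures and avoid blurry captures.
; Each item is then shown on its slot's mesh component, captured, drawn through a dynamic material and saved as a new or updated T_-prefixed Texture2D.
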(event Custom|Event_StartMainLoop
  (params (CDB :type Array%20of%20Customization%20Data%20Base%20Object%20References) (RenderTargets :type Array%20of%20Texture%20Render%20Target%202D%20Object%20References))
  ;[1 1 1] Update SkeletalMeshComponent target and capture
  (bind (_array_element _array_index) (Utilities|DelayedforEachLoop CDB (Variables|Default|GetDelayForLoop))
    (:Output
      (Rendering|SetVisibility (Variables|Default|GetWatch) false false)
      (Rendering|SetVisibility (Variables|Default|GetSkeletalMeshTarget) false false)
      (bind _rendertarget (CallFunction|GetSkeletalMeshComponentTargetfromCustomizationType _array_element))
      (bind _output_get (Variables|Default|SetSkeletalMeshTarget _rendertarget))
      (Rendering|SetVisibility _output_get true true)
      (bind _ascustomization_skeletal_mesh (Utilities|Casting|CastToCustomizationSkeletalMesh _array_element)
        (:then
          (CallFunction|ApplyCustomizationSkeletalMesh (Variables|Default|GetSkeletalMeshTarget) _ascustomization_skeletal_mesh))
        (:CastFailed
          (bind _ascustomization_skin (Utilities|Casting|CastToCustomizationSkin _array_element)
            (:then
              (CallFunction|ApplyCustomizationSkin (Variables|Default|GetSkeletalMeshTarget) _ascustomization_skin))
            (:CastFailed
              (bind _ascustomization_static_mesh (Utilities|Casting|CastToCustomizationStaticMesh _array_element))
              (Components|StaticMesh|SetStaticMesh (Variables|Default|GetWatch) (Utilities|ResolveSoftReference (Variables|/Script/ReadyOrNot.CustomizationStaticMesh|GetStaticMesh _ascustomization_static_mesh)))
              (Rendering|SetVisibility (Variables|Default|GetWatch) true true)))))
      (CallFunction|EventStartCapture (Utilities|String|Append "T_" (Utilities|GetObjectName _array_element)) RenderTargets _array_index))
    (:Complete
      (Components|SkinnedMesh|SetSkinnedAssetandUpdate (Variables|Default|GetSkeletalMeshTarget) 0 true)
      (Components|StaticMesh|SetStaticMesh (Variables|Default|GetWatch) 0))))

(event Custom|Event_StartCapture
  (params (TextureName :type String) (RenderTargets :type Array%20of%20Texture%20Render%20Target%202D%20Object%20References) (CurrentIndex :type Integer))
  (bind _camera (Variables|Default|GetCamera))
  ;[1 1 1] Capture scene and save to texture
  (bind _output_get (Variables|/Script/Engine.SceneCaptureComponent2D|SetTextureTarget (Variables|Default|GetCamera) (Utilities|Array|Get(acopy) RenderTargets CurrentIndex)))
  (Rendering|Material|SetTextureParameterValue (Variables|Default|GetDynamicRenderMaterial) "RenderTexture" _output_get)
  (Rendering|SceneCapture|CaptureScene _camera :!class /Script/Engine.SceneCaptureComponent2D)
  (Rendering|DrawMaterialtoRenderTarget (Variables|/Script/Engine.SceneCaptureComponent2D|GetTextureTarget _camera) (Variables|Default|GetDynamicRenderMaterial))
  (CallFunction|CreateStaticTexture (Variables|/Script/Engine.SceneCaptureComponent2D|GetTextureTarget _camera) TextureName (Utilities|Paths|GetPath (Class|KismetSystemLibrary|GetPathName (Variables|/Script/Engine.SceneCaptureComponent2D|GetTextureTarget _camera)))))

(event Custom|Event_StartPrepare
  (params (CDB :type Array%20of%20Customization%20Data%20Base%20Object%20References))
  (bind _temp_sm (Variables|Default|GetTEMP_SM))
  (bind _temp_watch (Variables|Default|GetTEMP_Watch))
  (bind _temp_sm_2 (Variables|Default|GetTEMP_SM))
  ;[1 1 1] Prepare all meshes and materials for fix blurry textures
  (for _array_element CDB
    (bind _ascustomization_skeletal_mesh (Utilities|Casting|CastToCustomizationSkeletalMesh _array_element)
      (:then
        (bind _object (Utilities|AsyncLoadAsset (Variables|/Script/ReadyOrNot.CustomizationSkeletalMesh|GetSkeletalMesh _ascustomization_skeletal_mesh))
          (:then
            _)
          (:Completed
            _))
        (bind _array_element_2 (Utilities|DelayedforEachLoop (Variables|/Script/ReadyOrNot.CustomizationSkeletalMesh|GetMaterialOverrides _ascustomization_skeletal_mesh) 0.1)
          (:Output
            (bind _object_2 (Utilities|AsyncLoadAsset (.Material (Utilities|Struct|BreakCustomizationMaterialSlot _array_element_2)))
              (:then
                _)
              (:Completed
                _))
            (bind _asskeletal_mesh (Utilities|Casting|CastToSkeletalMesh _object))
            (Components|SkinnedMesh|SetSkinnedAssetandUpdate _temp_sm_2 _asskeletal_mesh true)
            (bind _asmaterial_interface (Utilities|Casting|CastToMaterialInterface _object_2))
            (Rendering|Material|SetMaterial _temp_sm_2 (.Slot (Utilities|Struct|BreakCustomizationMaterialSlot _array_element_2)) _asmaterial_interface))
          (:Complete
            (bind _asskeletal_mesh_2 (Utilities|Casting|CastToSkeletalMesh _object))
            (Components|SkinnedMesh|SetSkinnedAssetandUpdate (Variables|Default|GetTEMP_SM) _asskeletal_mesh_2 true)))
        (Class|MeshComponent|PrestreamTextures (Variables|Default|GetTEMP_SM) (Variables|Default|GetDelayForLoop) false :!label _label))
      (:CastFailed
        (bind _ascustomization_skin (Utilities|Casting|CastToCustomizationSkin _array_element)
          (:then
            (bind _object_3 (Utilities|AsyncLoadAsset (Variables|/Script/ReadyOrNot.CustomizationSkin|GetMeshOverride _ascustomization_skin))
              (:then
                _)
              (:Completed
                _))
            (bind _array_element_3 (Utilities|DelayedforEachLoop (Variables|/Script/ReadyOrNot.CustomizationSkin|GetMaterialSlots _ascustomization_skin) 0.1)
              (:Output
                (bind _object_4 (Utilities|AsyncLoadAsset (.Material (Utilities|Struct|BreakCustomizationMaterialSlot _array_element_3)))
                  (:then
                    _)
                  (:Completed
                    _))
                (bind _asskeletal_mesh_3 (Utilities|Casting|CastToSkeletalMesh _object_3))
                (Components|SkinnedMesh|SetSkinnedAssetandUpdate _temp_sm _asskeletal_mesh_3 true)
                (bind _asmaterial_interface_2 (Utilities|Casting|CastToMaterialInterface _object_4))
                (Rendering|Material|SetMaterial _temp_sm (.Slot (Utilities|Struct|BreakCustomizationMaterialSlot _array_element_3)) _asmaterial_interface_2)
                (goto _label))
              (:Complete
                (bind _asskeletal_mesh_4 (Utilities|Casting|CastToSkeletalMesh _object_3))
                (Components|SkinnedMesh|SetSkinnedAssetandUpdate (Variables|Default|GetTEMP_SM) _asskeletal_mesh_4 true)
                (goto _label))))
          (:CastFailed
            (bind _ascustomization_static_mesh (Utilities|Casting|CastToCustomizationStaticMesh _array_element))
            (bind _object_5 (Utilities|AsyncLoadAsset (Variables|/Script/ReadyOrNot.CustomizationStaticMesh|GetStaticMesh _ascustomization_static_mesh))
              (:then
                _)
              (:Completed
                _))
            (bind _asstatic_mesh (Utilities|Casting|CastToStaticMesh _object_5))
            (Components|StaticMesh|SetStaticMesh _temp_watch _asstatic_mesh)
            (Class|MeshComponent|PrestreamTextures _temp_watch (Variables|Default|GetDelayForLoop) false)))))))

(event EventBeginPlay
  (bind _previewiconsdt (Variables|Default|GetPreviewIconsDT))
  ;[1 1 1] START
  (bind _outrownames (DataTable|GetDataTableRowNames _previewiconsdt))
  (bind _array_element (Utilities|DelayedforEachLoop _outrownames (Variables|Default|GetDelayForRow))
    (:Output
      (bind _returnvalue (Utilities|GetDataTableRow _previewiconsdt _array_element)
        (:then
          (Variables|Default|SetDelayForRow (* (Variables|Default|GetDelayForLoop) (+ (Utilities|Array|Length (.CDBs (Utilities|Struct|BreakPreviewIconsRow _returnvalue))) 1)))
          (CallFunction|EventStartPrepare (.CDBs (Utilities|Struct|BreakPreviewIconsRow _returnvalue)))
          (Utilities|FlowControl|Delay (Variables|Default|GetDelayForLoop))
          (CallFunction|EventStartMainLoop (.CDBs (Utilities|Struct|BreakPreviewIconsRow _returnvalue)) (.RenderTargets (Utilities|Struct|BreakPreviewIconsRow _returnvalue))))))))

(fn ConstructionScript
  ;[1 1 1] Create dynamic material for setting RenderTarget
  (bind _returnvalue (Rendering|Material|CreateDynamicMaterialInstance (Variables|Default|GetIconRenderMaterial) "None" "None" :!class /Script/Engine.KismetMaterialLibrary))
  (Rendering|Material|SetTextureParameterValue _returnvalue "RenderTexture" "/ReadyOrNot-CustomizationDataBase/Blueprints/IconGenerator/RenderTargets/RT_PreviewIcon_1024.RT_PreviewIcon_1024")
  (bind _output_get (Variables|Default|SetDynamicRenderMaterial _returnvalue))
  (Rendering|Material|SetMaterial (Variables|Default|GetIcon) 0 _output_get)
  (Variables|/Script/Engine.SceneCaptureComponent2D|SetTextureTarget (Variables|Default|GetCamera) "/ReadyOrNot-CustomizationDataBase/Blueprints/IconGenerator/RenderTargets/RT_PreviewIcon_1024.RT_PreviewIcon_1024"))

(fn ApplyCustomizationSkeletalMesh
  (params (TargetSkeletalMesh :type Skeletal%20Mesh%20Component%20Object%20Reference) (CDB_DA :type Customization%20Skeletal%20Mesh%20Object%20Reference))
  (bind _skeletalmesh (Variables|/Script/ReadyOrNot.CustomizationSkeletalMesh|GetSkeletalMesh CDB_DA))
  (if (Utilities|IsValidSoftObjectReference _skeletalmesh)
    (Components|SkinnedMesh|SetSkinnedAssetandUpdate TargetSkeletalMesh (Utilities|ResolveSoftReference _skeletalmesh) true)
    (CallFunction|ApplyMaterialsforMesh TargetSkeletalMesh (Variables|/Script/ReadyOrNot.CustomizationSkeletalMesh|GetMaterialOverrides CDB_DA))
    ;[1 1 1] Set CLEAR material for gloves
    (bind _ascustomization_gloves (Utilities|Casting|CastToCustomizationGloves CDB_DA))
    (Rendering|Material|SetMaterial TargetSkeletalMesh (Variables|/Script/ReadyOrNot.CustomizationGloves|GetSkinMaterialIndex _ascustomization_gloves) "/ReadyOrNot-CustomizationDataBase/Blueprints/IconGenerator/RenderTargets/M_CLEAR.M_CLEAR")))

(fn ApplyCustomizationSkin
  (params (TargetSkeletalMesh :type Skeletal%20Mesh%20Component%20Object%20Reference) (CS_DA :type Customization%20Skin%20Object%20Reference))
  (bind _meshoverride (Variables|/Script/ReadyOrNot.CustomizationSkin|GetMeshOverride CS_DA))
  (if (Utilities|IsValidSoftObjectReference _meshoverride)
    (Components|SkinnedMesh|SetSkinnedAssetandUpdate TargetSkeletalMesh (Utilities|ResolveSoftReference _meshoverride) true)
    (CallFunction|ApplyMaterialsforMesh TargetSkeletalMesh (Variables|/Script/ReadyOrNot.CustomizationSkin|GetMaterialSlots CS_DA))))

(fn ApplyMaterialsforMesh
  (params (SkeletalMesh :type Skeletal%20Mesh%20Component%20Object%20Reference) (CDB_Materials :type Array%20of%20Customization%20Material%20Slot%20Structures))
  (if (Utilities|IsValid SkeletalMesh)
    ;[1 1 1] Restore original materials
    (for (_array_element _array_index) (Variables|/Script/Engine.SkeletalMesh|GetMaterials (Variables|/Script/Engine.SkeletalMeshComponent|GetSkeletalMeshAsset SkeletalMesh))
      (Rendering|Material|SetMaterial SkeletalMesh _array_index (.MaterialInterface (Utilities|Struct|BreakSkeletalMaterial _array_element))))
    ;[1 1 1] Apply new materials
    (if (Utilities|Array|IsNotEmpty CDB_Materials)
      (for _array_element_2 CDB_Materials
        (Rendering|Material|SetMaterial SkeletalMesh (.Slot (Utilities|Struct|BreakCustomizationMaterialSlot _array_element_2)) (Utilities|ResolveSoftReference (.Material (Utilities|Struct|BreakCustomizationMaterialSlot _array_element_2))))))))

(fn CreateStaticTexture
  (params (TextureRenderTarget :type Texture%20Render%20Target%202D%20Object%20Reference) (TargetName :type String) (TargetFolder :type String))
  ;[1 1 1] Let's check if the current asset exists
  (bind _returnvalue (Class|AssetRegistry|GetAssetbyObjectPath(Message) (Utilities|ToObject(Interface) (Class|AssetRegistryHelpers|GetAssetRegistry)) (Utilities|String|StringToName (Utilities|String|Append TargetFolder "/" TargetName "." TargetName)) false))
  (bind _astexture_2d (Utilities|Casting|CastToTexture2D (Class|AssetRegistryHelpers|GetAsset _returnvalue))
    (:then
      ;[1 1 1] Update texture asset
      (EditorScripting|Rendering|ConvertRenderTargettoTexture2DEditorOnly TextureRenderTarget _astexture_2d))
    (:CastFailed
      ;[1 1 1] Create new asset
      (Class|KismetRenderingLibrary|RenderTargetCreateStaticTexture2DEditorOnly TextureRenderTarget TargetName (Variables|/Script/Engine.Texture|GetCompressionSettings _astexture_2d) "TMGS_NoMipmaps"))))

(fn GetSkeletalMeshComponentTargetfromCustomizationType
  (params (CustomizationType :type Customization%20Data%20Base%20Object%20Reference))
  (switch Utilities|FlowControl|Switch|SwitchonECustomizationType (Variables|/Script/ReadyOrNot.CustomizationDataBase|GetType CustomizationType)
    (:None
      (LocalVariables|SetRTarget 0 :!label _label)
      (return (LocalVariables|GetRTarget)))
    (:Character
      (goto _label))
    (:Voice
      (goto _label))
    (:Helmet
      (LocalVariables|SetRTarget (Variables|Default|GetHelmet))
      (return (LocalVariables|GetRTarget)))
    (:Shirt
      (LocalVariables|SetRTarget (Variables|Default|GetShirt))
      (return (LocalVariables|GetRTarget)))
    (:Pants
      (LocalVariables|SetRTarget (Variables|Default|GetPants))
      (return (LocalVariables|GetRTarget)))
    (:Shoes
      (LocalVariables|SetRTarget (Variables|Default|GetBoots))
      (return (LocalVariables|GetRTarget)))
    (:Eyewear
      (LocalVariables|SetRTarget (Variables|Default|GetGoggles))
      (return (LocalVariables|GetRTarget)))
    (:Belt
      (LocalVariables|SetRTarget (Variables|Default|GetBelt))
      (return (LocalVariables|GetRTarget)))
    (:Gloves
      (LocalVariables|SetRTarget (Variables|Default|GetGloves))
      (return (LocalVariables|GetRTarget)))
    (:Watch
      (goto _label))
    (:Tattoo
      (goto _label))
    (:PrimarySkin
      (goto _label))
    (:SecondarySkin
      (goto _label))
    (:ArmorSkin
      (LocalVariables|SetRTarget (Variables|Default|GetArmor))
      (return (LocalVariables|GetRTarget)))
    (:HelmetSkin
      (LocalVariables|SetRTarget (Variables|Default|GetHelmet)))
    (:HelmetMountSkin
      (LocalVariables|SetRTarget (Variables|Default|GetNightvision))
      (return (LocalVariables|GetRTarget)))
    (:FacewearSkin
      (LocalVariables|SetRTarget (Variables|Default|GetGoggles))
      (return (LocalVariables|GetRTarget)))
    (:Any
      (goto _label))))